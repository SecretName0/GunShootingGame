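; Wave-survival game mode for The Mercenary that spawns escalating minion waves, with periodic elite (Revenant or Wraith) and boss waves.
; GameStart sets wave size and runs a looping spawn timer, mostly placing AI at random navmesh points around the player.
; Tick detects cleared waves, swaps widgets, starts the next, and boosts player and enemy stats after elite and boss waves.
; Actors found in the level at BeginPlay serve as enemy stat templates.
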(event `self.ReceiveBeginPlay`
  (`self.Get Enemys Data`))

(event `Reset Time Event`
  ;[1 1 1] 추가 시간 UI발생 시 오프용
  (`KismetSystemLibrary.Delay` 1.0)
  (set `self.TimeBonus` 0.0))

(event `self.ReceiveTick`
  (params (DeltaSeconds :type "Float (single-precision)"))
  ;[1 1 1] 코멘트
  (if (`self.CanSpawn?`)
    _
    (elif (== (`self.RemainEnemy`) 0)
      (if (or (== (`self.WaveNum`) (- (`self.EliteWaveChecker`) 1)) (== (`self.WaveNum`) (- (`self.BossWaveChecker`) 1)))
        (if (`self.Sound Checker`)
          (`GameplayStatics.PlaySound2D` "/Engine/EditorSounds/GamePreview/EjectFromPlayer.EjectFromPlayer" 1.0 1.0 0.0 null null)
          (bind _returnvalue (`|CreateWidget` "/Game/UI/etc/WBP_EliteSpawn.WBP_EliteSpawn_C"))
          (`UserWidget.AddToViewport` _returnvalue 0)
          (set `self.Sound Checker` false)))
      (if (== (`self.WaveNum`) (`self.EliteWaveChecker`))
        (`self.Upgrade Enemy(Elite)`)
        (`self.Upgrade Ablity` 1.0 30.0) ; Elite Bonus
        (set `self.EliteWaveChecker` (+ (`self.EliteWaveChecker`) 3)) ; 스폰이 될 때마다 체커가 3라운드 후에 작동하도록 설정
        (set `self.Sound Checker` true)
        (elif (== (`self.WaveNum`) (`self.BossWaveChecker`))
          (`self.Upgrade Ablity` 3.0 50.0) ; Boss Bonus
          (set `self.BossWaveChecker` (+ (`self.BossWaveChecker`) 10))
          (`self.Upgrade Enemy(Boss)`)
          (set `self.Sound Checker` true)
          (else
            (bind _returnvalue_2 (`|CreateWidget` "/Game/UI/etc/WBP_WaveClear.WBP_WaveClear_C"))
            (`UserWidget.AddToViewport` _returnvalue_2 0)
            (`KismetSystemLibrary.Delay` 3.0) ; Nothing
            (`WidgetLayoutLibrary.RemoveAllWidgets`)
            (if (`self.IsWraith?`)
              (bind _returnvalue_3 (`|CreateWidget` "/Game/UI/HUD/Mercenary_HUD/WBP_HUD_Wraith_TM.WBP_HUD_Wraith_TM_C"))
              (`UserWidget.AddToViewport` _returnvalue_3 0)
              (`self.Game Start`)
              (else
                (bind _returnvalue_4 (`|CreateWidget` "/Game/UI/HUD/Mercenary_HUD/WBP_HUD_Rev_TM.WBP_HUD_Rev_TM_C"))
                (`UserWidget.AddToViewport` _returnvalue_4 0)
                (`self.Game Start`)))))))))

(event `Game Start`
  ;[1 1 1] 코멘트
  (set `self.CanSpawn?` true)
  (`|ExecutionSequence`
    (:`then_0`
      (`/Engine/EditorBlueprintResources/StandardMacros.IncrementInt` (`self.WaveNum`)
        (:`  `
          (if (<= (`self.WaveNum`) 3)
            (bind _output_get (set `self.MaxSpawn` 5))
            (set `self.RemainEnemy` _output_get)
            (elif (<= (`self.WaveNum`) 5)
              (bind _output_get_2 (set `self.MaxSpawn` 7))
              (set `self.RemainEnemy` _output_get_2)
              (elif (<= (`self.WaveNum`) 10)
                (bind _output_get_3 (set `self.MaxSpawn` 10))
                (set `self.RemainEnemy` _output_get_3)
                (elif (<= (`self.WaveNum`) 99)
                  (set `self.MaxSpawn` (* (`self.웨이브별 증량 몹`) (`self.웨이브 추가`)))
                  (`/Engine/EditorBlueprintResources/StandardMacros.IncrementInt` (`self.웨이브 추가`)))))))))
    (:`then_1`
      (`KismetSystemLibrary.K2_SetTimer` null "Spawn_Minion" (`KismetMathLibrary.RandomFloatInRange` 1.0 3.0) true))
    (:`then_2`
      (if (== (`self.WaveNum`) (`self.EliteWaveChecker`))
        (`self.Spawn_Elite`)))
    (:`then_3`
      (if (== (`self.WaveNum`) (`self.BossWaveChecker`))
        (`self.Spawn_Boss`)))))

(fn `Enemy Spawn Rule`
  (params (`Spawn Class` :type "Pawn Class Reference"))
  (returns (`Spawn Pawn Object Reference` :type "Pawn Object Reference"))
  (bind _randomlocation (`NavigationSystemV1.K2_GetRandomLocationInNavigableRadius` (`self.K2_GetActorLocation` (`GameplayStatics.GetPlayerPawn` 0)) 5000.0 null null))
  (bind _returnvalue (`AIBlueprintHelperLibrary.SpawnAIFromClass` `Spawn Class` "/Game/Blueprints/Characters/E_EnemyController/SpawnType/BT_Enemys_AI_Sp.BT_Enemys_AI_Sp" _randomlocation (struct) false null))
  (return _returnvalue))

(fn `Get Enemys Data`
  (`|ExecutionSequence`
    (:`then_0`
      (bind _returnvalue (`GameplayStatics.GetActorOfClass` "/Game/Blueprints/Characters/B_Minion/BP_Minion_Siege_TM.BP_Minion_Siege_TM_C"))
      (bind _output_get (set `self.Minion Data` _returnvalue))
      (set `self.Minion` (`GameplayStatics.GetObjectClass` _output_get)))
    (:`then_1`
      (bind _returnvalue_2 (`GameplayStatics.GetActorOfClass` "/Game/Blueprints/Characters/A_Wraith/BP_Wraith_TM.BP_Wraith_TM_C"))
      (bind _output_get_2 (set `self.Wraith Data` _returnvalue_2))
      (set `self.Wraith` (`GameplayStatics.GetObjectClass` _output_get_2)))
    (:`then_2`
      (bind _returnvalue_3 (`GameplayStatics.GetActorOfClass` "/Game/Blueprints/Characters/A_Revenant/BP_Revenant_TM.BP_Revenant_TM_C"))
      (bind _output_get_3 (set `self.Revenant Data` _returnvalue_3))
      (set `self.Rev` (`GameplayStatics.GetObjectClass` _output_get_3)))
    (:`then_3`
      (bind _returnvalue_4 (`GameplayStatics.GetActorOfClass` "/Game/Blueprints/Characters/B_Boss/BP_HellTaker_TM.BP_HellTaker_TM_C"))
      (bind _output_get_4 (set `self.Boss Data` _returnvalue_4))
      (set `self.Boss` (`GameplayStatics.GetObjectClass` _output_get_4)))))

(fn `Get Player Data`
  (bind _asbase_character (cast `BaseCharacter` (`GameplayStatics.GetPlayerPawn` 0)))
  (set `self.Player Data` _asbase_character))

(fn `Spawn_Boss`
  (locals (`Local Boss` :type "/Game/Blueprints/Characters/B_Boss/BP_HellTaker_TM Object Reference"))
  (bind _boss_data (`self.Boss Data`))
  (bind _spawn_pawn_object_reference (`self.Enemy Spawn Rule` (`self.Boss`)))
  (bind _asbp_hell_taker (cast `/Game/Blueprints/Characters/B_Boss/BP_HellTaker_TM` _spawn_pawn_object_reference))
  (bind _output_get (set `local.Local Boss` _asbp_hell_taker))
  (bind _output_get_2 (set `BaseCharacter.Max_HP` (`BaseCharacter.Max_HP` _boss_data) _output_get))
  (set `BaseCharacter.HP` _output_get_2 _output_get)
  (set `BaseCharacter.GunDamage` (`HellTaker.Boss_ATK` _boss_data) _output_get))

(fn `Spawn_Elite`
  (locals (`Local Rev` :type "/Game/Blueprints/Characters/A_Revenant/BP_Revenant_TM Object Reference") (`Local Wraith` :type "/Game/Blueprints/Characters/A_Wraith/BP_Wraith_TM Object Reference"))
  (bind _revenant_data (`self.Revenant Data`))
  (bind _wraith_data (`self.Wraith Data`))
  (bind _randomlocation (`NavigationSystemV1.K2_GetRandomLocationInNavigableRadius` (`self.K2_GetActorLocation` (`GameplayStatics.GetPlayerPawn` 0)) 5000.0 null null))
  (if (== (`KismetMathLibrary.RandomIntegerInRange` 1 2) 1)
    (bind _returnvalue (`AIBlueprintHelperLibrary.SpawnAIFromClass` "/Game/Blueprints/Characters/A_Revenant/BP_Revenant_TM.BP_Revenant_TM_C" "/Game/Blueprints/Characters/E_EnemyController/SpawnType/BT_Enemys_AI_Sp.BT_Enemys_AI_Sp" _randomlocation (struct) false null))
    (bind _asbp_revenant_tm (cast `/Game/Blueprints/Characters/A_Revenant/BP_Revenant_TM` _returnvalue))
    (bind _output_get (set `local.Local Rev` _asbp_revenant_tm))
    (bind _output_get_2 (set `BaseCharacter.HP` (`BaseCharacter.Max_HP` _revenant_data) _output_get))
    (set `BaseCharacter.Max_HP` _output_get_2 _output_get)
    (set `BaseCharacter.GunDamage` (`Revenant.R_ATK` _revenant_data) _output_get)
    (else
      (bind _returnvalue_2 (`AIBlueprintHelperLibrary.SpawnAIFromClass` "/Game/Blueprints/Characters/A_Wraith/BP_Wraith_TM.BP_Wraith_TM_C" "/Game/Blueprints/Characters/E_EnemyController/SpawnType/BT_Enemys_AI_Sp.BT_Enemys_AI_Sp" (0.0 0.0 0.0) (struct) false null))
      (bind _asbp_wraith_tm (cast `/Game/Blueprints/Characters/A_Wraith/BP_Wraith_TM` _returnvalue_2))
      (bind _output_get_3 (set `local.Local Wraith` _asbp_wraith_tm))
      (bind _output_get_4 (set `BaseCharacter.HP` (`BaseCharacter.Max_HP` _wraith_data) _output_get_3))
      (set `BaseCharacter.Max_HP` _output_get_4 _output_get_3)
      (set `BaseCharacter.GunDamage` (`Wraith.W_ATK` _wraith_data) _output_get_3))))

(fn `Spawn_Minion`
  (bind _maxspawn (`self.MaxSpawn`))
  (bind _upgrade_enemy_hp_minion (`self.UPGRADE Enemy HP Minion`))
  (bind _spawn_pawn_object_reference (`self.Enemy Spawn Rule` (`self.Minion`)))
  (bind _asbp_minion_siege_tm (cast `/Game/Blueprints/Characters/B_Minion/BP_Minion_Siege_TM` _spawn_pawn_object_reference))
  (set `BaseCharacter.Max_HP` _upgrade_enemy_hp_minion _asbp_minion_siege_tm)
  (set `BaseCharacter.HP` _upgrade_enemy_hp_minion _asbp_minion_siege_tm)
  (set `BaseCharacter.GunDamage` (`self.UPGRADE Enemy ATK_Min`) _asbp_minion_siege_tm)
  (`/Engine/EditorBlueprintResources/StandardMacros.IncrementInt` (`self.SpawnedNum`)
    (:`  `
      (`/Engine/EditorBlueprintResources/StandardMacros.DecrementInt` _maxspawn
        (:`  `
          (if (not (> _maxspawn 0))
            (`KismetSystemLibrary.K2_ClearTimer` null "Spawn_Minion")
            (set `self.CanSpawn?` false)))))))

(fn `Upgrade Ablity`
  (params (`Bonus Power` :type "Float (double-precision)") (`Bonus HP` :type "Float (double-precision)"))
  (bind _player_data (`self.Player Data`))
  (bind _player_data_2 (`self.Player Data`))
  (bind _player_data_3 (`self.Player Data`))
  (if (`self.ActorHasTag` (`self.Player Data`) "Player")
    (set `BaseCharacter.GunDamage` (+ (`BaseCharacter.GunDamage` _player_data_2) `Bonus Power`) _player_data_2)
    (set `BaseCharacter.Max_HP` (+ (`BaseCharacter.Max_HP` _player_data_3) `Bonus HP`) _player_data_3)
    (set `BaseCharacter.HP` (+ (`BaseCharacter.HP` _player_data) `Bonus HP`) _player_data)))

(fn `Upgrade Enemy Calculating End Of Boss Stage`
  (bind _revenant_data (`self.Revenant Data`))
  (bind _boss_data (`self.Boss Data`))
  (bind _wraith_data (`self.Wraith Data`))
  (set `self.UPGRADE Enemy HP Minion` (* (`Minion.MW_HP` (`self.Minion Data`)) 1.1))
  (set `self.UPGRADE Enemy ATK_Min` (* (`Minion.ATK` (`self.Minion Data`)) 1.1))
  (set `BaseCharacter.Max_HP` (* (`BaseCharacter.Max_HP` _wraith_data) 1.1) _wraith_data)
  (set `Wraith.W_ATK` (* (`Wraith.W_ATK` _wraith_data) 1.1) _wraith_data)
  (set `BaseCharacter.Max_HP` (* (`BaseCharacter.Max_HP` _revenant_data) 1.1) _revenant_data)
  (set `Revenant.R_ATK` (* (`Revenant.R_ATK` _revenant_data) 1.1) _revenant_data)
  (set `BaseCharacter.Max_HP` (* (`BaseCharacter.Max_HP` _boss_data) 1.2) _boss_data)
  (set `HellTaker.Boss_ATK` (* (`HellTaker.Boss_ATK` _boss_data) 1.2) _boss_data))

(fn `Upgrade Enemy Calculating End Of Elite Stage`
  (bind _revenant_data (`self.Revenant Data`))
  (bind _wraith_data (`self.Wraith Data`))
  (set `self.UPGRADE Enemy HP Minion` (* (`Minion.MW_HP` (`self.Minion Data`)) 1.05))
  (set `BaseCharacter.Max_HP` (* (`BaseCharacter.Max_HP` _wraith_data) 1.05) _wraith_data)
  (set `BaseCharacter.Max_HP` (* (`BaseCharacter.Max_HP` _revenant_data) 1.05) _revenant_data))

(fn `Upgrade Enemy(Boss)`
  (`self.Upgrade Enemy Calculating End Of Boss Stage`)
  (bind _output_get (set `BaseCharacter.Max_HP` (`self.UPGRADE Enemy HP Minion`) (`self.Minion Data`)))
  (bind _output_get_2 (set `BaseCharacter.HP` _output_get (`self.Minion Data`))) ; 이미 스폰이 되어있는 미니언에게 적용
  (set `Minion.MW_HP` _output_get_2 (`self.Minion Data`)))

(fn `Upgrade Enemy(Elite)`
  (`self.Upgrade Enemy Calculating End Of Elite Stage`) ; 업글될 때마다 미리 계산
  (bind _output_get (set `BaseCharacter.Max_HP` (`self.UPGRADE Enemy HP Minion`) (`self.Minion Data`)))
  (bind _output_get_2 (set `BaseCharacter.HP` _output_get (`self.Minion Data`))) ; 이미 스폰이 되어있는 미니언에게 적용
  (set `Minion.MW_HP` _output_get_2 (`self.Minion Data`)))

(fn `UserConstructionScript`)