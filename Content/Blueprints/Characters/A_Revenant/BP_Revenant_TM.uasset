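; Revenant character Blueprint for a timed, scored game mode, serving as player or enemy by actor tag.
; BeginPlay hides the HP widget and caches BP_TheMercenary only for Player-tagged actors; Tick refreshes the HP bar.
; On an enemy's death, Tick once adds random bonus time and score through the game mode, then despawns after a delay.
; The random item drop calls an empty function, as its potion-spawning nodes are disconnected.
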(event `self.ReceiveBeginPlay`
  ;[1 1 1] Begin
  (if (`self.ActorHasTag` "Player")
    (`SceneComponent.SetHiddenInGame` (`self.HP Widget`) true false)
    (`self.Get Game Mode`)))

(event `self.ReceiveTick`
  (params (DeltaSeconds :type "Float (single-precision)"))
  (`self.SetPercent`)
  (if (and (`self.bIsDead`) (`self.ActorHasTag` "Enemy") (`self.Dead Checker`))
    (set `self.Dead Checker` false)
    (`self.PlusTime`)
    (`self.Score Get`)
    (if (`KismetMathLibrary.RandomBool`)
      (`self.Drop Item`)
      (`KismetSystemLibrary.Delay` 1.5)
      (`self.DeSpawn`)
      (else
        (`KismetSystemLibrary.Delay` 1.5)
        (`self.DeSpawn`)))))

(fn `Drop Item`)

(fn `Enemy Death`)

(fn `Get Game Mode`
  (bind _asbp_the_mercenary (cast `/Game/Blueprints/GameMode/BP_TheMercenary` (`GameplayStatics.GetGameMode`)))
  (set `self.The Mercenary` _asbp_the_mercenary))

(fn `PlusTime`
  (bind _asbp_the_mercenary (cast `/Game/Blueprints/GameMode/BP_TheMercenary` (`GameplayStatics.GetGameMode`)))
  (bind _output_get (set `TheMercenary.TimeBonus` (`KismetMathLibrary.Conv_IntToDouble` (`KismetMathLibrary.RandomIntegerInRange` 3 5)) _asbp_the_mercenary))
  (set `TheMercenary.RemainTime` (+ (`TheMercenary.RemainTime` _asbp_the_mercenary) _output_get) _asbp_the_mercenary))

(fn `Score Get`
  (bind _the_mercenary (`self.The Mercenary`))
  (set `TheMercenary.Score` (+ (`TheMercenary.Score` _the_mercenary) (`self.Death Score`)) _the_mercenary))

(fn `SetPercent`
  (bind _aswbp_enemy_hp (cast `/Game/UI/etc/WBP_Enemy_HP` (`WidgetComponent.GetWidget` (`self.HP Widget`))))
  (`ProgressBar.SetPercent` (`/Game/UI/etc/WBP_Enemy_HP.HPratio` _aswbp_enemy_hp) (/ (`self.HP`) (`self.Max_HP`))))

(fn `UserConstructionScript`)