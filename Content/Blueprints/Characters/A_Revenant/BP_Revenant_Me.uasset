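; BP_Revenant_Me is the Revenant character Blueprint, usable as a player or enemy depending on its actor tag.
; On BeginPlay it hides the overhead HP widget for the player-tagged instance.
; Each tick it sets the WBP_Enemy_HP bar to HP over MaxHP.
; When an enemy-tagged instance dies, a one-shot check gives it a random chance to despawn after a short delay.
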(event `self.ReceiveBeginPlay`
  ;[1 1 1] Begin
  (if (`self.ActorHasTag` "Player")
    (`SceneComponent.SetHiddenInGame` (`self.HP Widget`) true false)))

(event `self.ReceiveTick`
  (params (DeltaSeconds :type "Float (single-precision)"))
  (`self.SetPercent`)
  (if (and (`self.bIsDead`) (`self.ActorHasTag` "Enemy") (`self.Dead Checker`))
    (set `self.Dead Checker` false)
    (if (`KismetMathLibrary.RandomBool`)
      (`KismetSystemLibrary.Delay` 1.5)
      (`self.DeSpawn`))))

(fn `SetPercent`
  (bind _aswbp_enemy_hp (cast `/Game/UI/etc/WBP_Enemy_HP` (`WidgetComponent.GetWidget` (`self.HP Widget`))))
  (`ProgressBar.SetPercent` (`/Game/UI/etc/WBP_Enemy_HP.HPratio` _aswbp_enemy_hp) (/ (`self.HP`) (`self.Max_HP`))))

(fn `UserConstructionScript`)