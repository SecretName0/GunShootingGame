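; BP_HellTaker_TM is a boss character for the BP_TheMercenary game mode that awards extra time when it dies.
; It sets its walk speed at BeginPlay and refreshes its HP widget bar every Tick from the HP ratio.
; Tick also polls for death, using DeadChecker as a one-shot gate to add a fixed bonus to the game mode's remaining time, then despawns after a short delay.
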(event `self.ReceiveBeginPlay`
  (set `CharacterMovementComponent.MaxWalkSpeed` 800.0 (`self.CharacterMovement`)))

(event `self.ReceiveTick`
  (params (DeltaSeconds :type "Float (single-precision)"))
  (`self.SetPercent`)
  (if (and (`self.bIsDead`) (`self.Dead Checker`))
    (set `self.Dead Checker` false)
    (`self.PlusTimer`)
    (`KismetSystemLibrary.Delay` 1.0)
    (`self.DeSpawn`)))

(fn `PlusTimer`
  (bind _asbp_the_mercenary (cast `/Game/Blueprints/GameMode/BP_TheMercenary` (`GameplayStatics.GetGameMode`)))
  (bind _output_get (set `TheMercenary.TimeBonus` (`KismetMathLibrary.Conv_IntToDouble` (`KismetMathLibrary.RandomIntegerInRange` 10 10)) _asbp_the_mercenary))
  (set `TheMercenary.RemainTime` (+ (`TheMercenary.RemainTime` _asbp_the_mercenary) _output_get) _asbp_the_mercenary))

(fn `SetPercent`
  (bind _aswbp_enemy_hp (cast `/Game/UI/etc/WBP_Enemy_HP` (`WidgetComponent.GetWidget` (`self.HP_Widget`))))
  (`ProgressBar.SetPercent` (`/Game/UI/etc/WBP_Enemy_HP.HPratio` _aswbp_enemy_hp) (/ (`self.HP`) (`self.Max_HP`))))

(fn `UserConstructionScript`)