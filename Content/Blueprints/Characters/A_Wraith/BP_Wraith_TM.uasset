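; Wraith character for the TheMercenary game mode, serving as player or enemy according to its actor tag.
; Dash raises walk speed while W is held, and the player variant hides its HP bar.
; Tick refreshes the HP bar and handles enemy death once, adding random bonus time and score, randomly dropping one of three potions, then despawning after a delay.
; The game mode reference used for scoring is cached only on Player-tagged instances.
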(event `Key|W`
  (params (Key :type "Key Structure"))
  ;[1 1 1] Dash
  (:`Pressed`
    (set `self.Pressed  W` true))
  (:`Released`
    (set `self.Pressed  W` false)))

(event `InputAction|Dash`
  (params (Key :type "Key Structure"))
  (bind _charactermovement (`self.CharacterMovement`))
  ;[1 1 1] Dash
  (:`Pressed`
    (if (`self.Pressed  W`)
      (set `self.IsDash` true)
      (set `CharacterMovementComponent.MaxWalkSpeed` (* (`CharacterMovementComponent.MaxWalkSpeed` _charactermovement) (`self.Dash Speed`)) _charactermovement)))
  (:`Released`
    (set `self.IsDash` false)
    (set `CharacterMovementComponent.MaxWalkSpeed` 600.0 (`self.CharacterMovement`))))

(event `self.ReceiveBeginPlay`
  ;[1 1 1] Begin
  (if (`self.ActorHasTag` "Player")
    (`SceneComponent.SetHiddenInGame` (`self.HPWidget`) true false)
    (`self.Get Mode Data`)))

(event `self.ReceiveTick`
  (params (DeltaSeconds :type "Float (single-precision)"))
  (`self.SetPercent`)
  (if (and (`self.bIsDead`) (`self.ActorHasTag` "Enemy") (`self.Dead Checker`))
    (set `self.Dead Checker` false)
    (`self.Plus TImer`)
    (`self.Score Get`)
    (if (`KismetMathLibrary.RandomBool`)
      (`self.DropItem`)
      (`KismetSystemLibrary.Delay` 1.5)
      (`self.DeSpawn`)
      (else
        (`KismetSystemLibrary.Delay` 1.5)
        (`self.DeSpawn`)))))

(fn `DropItem`
  (bind _output_get (set `self.Random Item` (`KismetMathLibrary.RandomInteger` 3)))
  (if (== _output_get 0)
    (`|SpawnActorFromClass` "/Game/Blueprints/Actors/BP_HPPotion.BP_HPPotion_C" (`KismetMathLibrary.Conv_VectorToTransform` (`self.K2_GetActorLocation`)) "Undefined" "MultiplyWithRoot" null null)
    (elif (== _output_get 1)
      (`|SpawnActorFromClass` "/Game/Blueprints/Actors/BP_DotPotion.BP_DotPotion_C" (`KismetMathLibrary.Conv_VectorToTransform` (`self.K2_GetActorLocation`)) "Undefined" "MultiplyWithRoot" null null)
      (elif (== _output_get 2)
        (`|SpawnActorFromClass` "/Game/Blueprints/Actors/BP_AtkPotion.BP_AtkPotion_C" (`KismetMathLibrary.Conv_VectorToTransform` (`self.K2_GetActorLocation`)) "Undefined" "MultiplyWithRoot" null null)))))

(fn `Enemy Death`)

(fn `Get Mode Data`
  (bind _asbp_the_mercenary (cast `/Game/Blueprints/GameMode/BP_TheMercenary` (`GameplayStatics.GetGameMode`)))
  (set `self.The Mercenary` _asbp_the_mercenary))

(fn `Plus TImer`
  (bind _asbp_the_mercenary (cast `/Game/Blueprints/GameMode/BP_TheMercenary` (`GameplayStatics.GetGameMode`)))
  (bind _output_get (set `TheMercenary.TimeBonus` (`KismetMathLibrary.Conv_IntToDouble` (`KismetMathLibrary.RandomIntegerInRange` 3 5)) _asbp_the_mercenary))
  (set `TheMercenary.RemainTime` (+ (`TheMercenary.RemainTime` _asbp_the_mercenary) _output_get) _asbp_the_mercenary))

(fn `Score Get`
  (bind _the_mercenary (`self.The Mercenary`))
  (set `TheMercenary.Score` (+ (`TheMercenary.Score` _the_mercenary) (`self.Death Score`)) _the_mercenary))

(fn `SetPercent`
  (bind _aswbp_enemy_hp (cast `/Game/UI/etc/WBP_Enemy_HP` (`WidgetComponent.GetWidget` (`self.HPWidget`))))
  (`ProgressBar.SetPercent` (`/Game/UI/etc/WBP_Enemy_HP.HPratio` _aswbp_enemy_hp) (/ (`self.HP`) (`self.Max_HP`))))

(fn `UserConstructionScript`)