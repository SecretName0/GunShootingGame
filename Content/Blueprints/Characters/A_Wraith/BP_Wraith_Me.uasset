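; Wraith character Blueprint that handles dashing, an HP bar widget and despawning, branching on Player and Enemy tags.
; Pressing Dash while W is held multiplies walk speed by DashSpeed, and releasing it resets to a hardcoded default.
; The HP widget is hidden for the player and refreshed every Tick.
; Tick also despawns dead enemies once after a short delay, gated by DeadChecker.
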(event `Key|W`
  (params (Key :type "Key Structure"))
  ;[1 1 1] Dash
  (:`Pressed`
    (set `self.Pressed  W` true))
  (:`Released`
    (set `self.Pressed  W` false)))

(event `InputAction|Dash`
  (params (Key :type "Key Structure"))
  (bind _charactermovement (`self.CharacterMovement`))
  ;[1 1 1] Dash
  (:`Pressed`
    (if (`self.Pressed  W`)
      (set `self.IsDash` true)
      (set `CharacterMovementComponent.MaxWalkSpeed` (* (`CharacterMovementComponent.MaxWalkSpeed` _charactermovement) (`self.Dash Speed`)) _charactermovement)))
  (:`Released`
    (set `self.IsDash` false)
    (set `CharacterMovementComponent.MaxWalkSpeed` 600.0 (`self.CharacterMovement`))))

(event `self.ReceiveBeginPlay`
  ;[1 1 1] Begin
  (if (`self.ActorHasTag` "Player")
    (`SceneComponent.SetHiddenInGame` (`self.HPWidget`) true false)))

(event `self.ReceiveTick`
  (params (DeltaSeconds :type "Float (single-precision)"))
  (`self.SetPercent`)
  (if (and (`self.bIsDead`) (`self.ActorHasTag` "Enemy") (`self.Dead Checker`))
    (set `self.Dead Checker` false)
    (`KismetSystemLibrary.Delay` 1.5)
    (`self.DeSpawn`)))

(fn `SetPercent`
  (bind _aswbp_enemy_hp (cast `/Game/UI/etc/WBP_Enemy_HP` (`WidgetComponent.GetWidget` (`self.HPWidget`))))
  (`ProgressBar.SetPercent` (`/Game/UI/etc/WBP_Enemy_HP.HPratio` _aswbp_enemy_hp) (/ (`self.HP`) (`self.Max_HP`))))

(fn `UserConstructionScript`)