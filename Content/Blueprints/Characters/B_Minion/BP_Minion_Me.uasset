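; BP_Minion_Me is a minion character Blueprint that shows its health and despawns shortly after death.
; Every Tick it casts the HPWidget component's widget to WBP_Enemy_HP and sets the HPratio bar to HP divided by MaxHP.
; Once IsDead is set, the DeadChecker flag lets a short delay and DeSpawn call run only once.
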(event `self.ReceiveTick`
  (params (DeltaSeconds :type "Float (single-precision)"))
  (`self.SetPercent`)
  (if (and (`self.bIsDead`) (`self.Dead Checker`))
    (set `self.Dead Checker` false)
    (`KismetSystemLibrary.Delay` 0.5)
    (`self.DeSpawn`)))

(fn `SetPercent`
  (bind _aswbp_enemy_hp (cast `/Game/UI/etc/WBP_Enemy_HP` (`WidgetComponent.GetWidget` (`self.HP_Widget`))))
  (`ProgressBar.SetPercent` (`/Game/UI/etc/WBP_Enemy_HP.HPratio` _aswbp_enemy_hp) (/ (`self.HP`) (`self.Max_HP`))))

(fn `UserConstructionScript`)