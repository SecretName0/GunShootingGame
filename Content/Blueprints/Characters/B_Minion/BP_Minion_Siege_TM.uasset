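; Siege minion enemy for The Mercenary game mode that rewards the player with time and score when it dies.
; Tick refreshes the overhead HP bar and uses a one-shot flag to catch death.
; Death adds a random time bonus and its score to the cached game mode, then randomly may spawn an HP, Dot or Atk potion before a delayed despawn.
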(event `self.ReceiveBeginPlay`
  (bind _asbp_the_mercenary (cast `/Game/Blueprints/GameMode/BP_TheMercenary` (`GameplayStatics.GetGameMode`)))
  (set `self.Mercenary Mode` _asbp_the_mercenary))

(event `self.ReceiveTick`
  (params (DeltaSeconds :type "Float (single-precision)"))
  (`self.SetPercent`)
  (if (and (`self.bIsDead`) (`self.Dead Checker`))
    (set `self.Dead Checker` false)
    (`self.Plus Timer`)
    (`self.Score Get`)
    (if (`KismetMathLibrary.RandomBool`)
      (`self.Drop Item`)
      (`KismetSystemLibrary.Delay` 0.5)
      (`self.DeSpawn`)
      (else
        (`KismetSystemLibrary.Delay` 0.5)
        (`self.DeSpawn`)))))

(fn `Drop Item`
  (bind _output_get (set `self.Random Item` (`KismetMathLibrary.RandomInteger` 4)))
  (if (<= _output_get 1)
    (`|SpawnActorFromClass` "/Game/Blueprints/Actors/BP_HPPotion.BP_HPPotion_C" (`KismetMathLibrary.Conv_VectorToTransform` (`self.K2_GetActorLocation`)) "Undefined" "MultiplyWithRoot" null null)
    (elif (== _output_get 2)
      (`|SpawnActorFromClass` "/Game/Blueprints/Actors/BP_DotPotion.BP_DotPotion_C" (`KismetMathLibrary.Conv_VectorToTransform` (`self.K2_GetActorLocation`)) "Undefined" "MultiplyWithRoot" null null)
      (elif (== _output_get 3)
        (`|SpawnActorFromClass` "/Game/Blueprints/Actors/BP_AtkPotion.BP_AtkPotion_C" (`KismetMathLibrary.Conv_VectorToTransform` (`self.K2_GetActorLocation`)) "Undefined" "MultiplyWithRoot" null null)))))

(fn `Plus Timer`
  (bind _mercenary_mode (`self.Mercenary Mode`))
  (bind _output_get (set `TheMercenary.TimeBonus` (`KismetMathLibrary.Conv_IntToDouble` (`KismetMathLibrary.RandomIntegerInRange` 3 5)) _mercenary_mode))
  (set `TheMercenary.RemainTime` (+ (`TheMercenary.RemainTime` _mercenary_mode) _output_get) _mercenary_mode))

(fn `Score Get`
  (bind _mercenary_mode (`self.Mercenary Mode`))
  (set `/Game/Blueprints/GameMode/BP_TheMercenary.Score` (+ (`/Game/Blueprints/GameMode/BP_TheMercenary.Score` _mercenary_mode) (`self.Death Score`)) _mercenary_mode))

(fn `SetPercent`
  (bind _aswbp_enemy_hp (cast `/Game/UI/etc/WBP_Enemy_HP` (`WidgetComponent.GetWidget` (`self.HP_Widget`))))
  (`ProgressBar.SetPercent` (`/Game/UI/etc/WBP_Enemy_HP.HPratio` _aswbp_enemy_hp) (/ (`self.HP`) (`self.Max_HP`))))

(fn `UserConstructionScript`)